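; BP_Projectile is a player projectile that can be recalled to the player who fires it.
; Calling ReturnToPlayer sets a flag that makes Tick halt the ProjectileMovement component and ease the actor toward the player pawn with VInterpTo.
; Once within a small radius of the player, it destroys itself and re-enables CanShoot on BP_Player.
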(event EventTick
  (params (DeltaSeconds :type Float%20%28single-precision%29))
  (bind _returnvalue (Game|Player|GetPlayerPawn 0))
  (bind _returnvalue_2 (Transformation|GetActorLocation))
  (bind _returnvalue_3 (Transformation|GetActorLocation _returnvalue))
  (if (Variables|Default|GetbReturnToPlayer)
    (Components|Movement|StopMovementImmediately (Variables|Default|GetProjectileMovement))
    (Transformation|SetActorLocation (Math|Interpolation|VInterpTo _returnvalue_2 _returnvalue_3 DeltaSeconds 4.0) false false)
    (if (Math|Vector|Equal(Vector) _returnvalue_2 _returnvalue_3 75.0)
      (Actor|DestroyActor)
      (bind _asbp_player (Utilities|Casting|CastToBP_Player (Game|GetPlayerCharacter 0)))
      (Variables|/Game/Blueprints/BP_Player.BP_Player_C|SetbCanShoot _asbp_player true))))

(fn ConstructionScript)

(fn ReturntoPlayer
  (Variables|Default|SetbReturnToPlayer true))