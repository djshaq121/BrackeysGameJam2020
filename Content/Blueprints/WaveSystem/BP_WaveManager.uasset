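; BP_WaveManager runs enemy waves from data table rows keyed by wave number, ending when no row remains.
; After each countdown, a looping timer spawns that row's enemy groups at random ground spawn points gathered on BeginPlay, casting each class to BP_ThrowingEnemy.
; Spawned enemies receive a manager reference; EnemyDead tallies kills and restarts the countdown once all are dead.
; An older polling check for dead enemies remains disconnected.
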(event Custom|Start%20Countdown
  (bind _allwavecomplete (CallFunction|GameComplete))
  (if _allwavecomplete
    (Development|PrintString "All waves complete")
    (else
      ;[1 1 1] Countdown
      (bind _returnvalue (Utilities|Time|SetTimerbyEvent (delegate Custom|Count) 1.0 true))
      (Variables|Default|SetTime 5))))

(event Custom|Count
  ;[1 1 1] Countdown
  (if (== (Variables|Default|GetTime) 0)
    (Utilities|Time|ClearandInvalidateTimerbyHandle (stale Custom|Start%20Countdown _returnvalue))
    (CallFunction|BeginWave)
    (else
      (Math|Integer|DecrementInt (Variables|Default|GetTime)))))

(event Custom|Begin%20Wave
  (bind _returnvalue (Utilities|GetDataTableRow (Variables|Default|GetEnemyDataTable) (Utilities|String|StringToName (Utilities|String|ToString(Integer) (Variables|Default|GetWaveCounter))))
    (:then
      (Variables|Default|SetCurrentWaveInfo (Utilities|Struct|BreakWaveInfo _returnvalue))
      (Variables|Default|SetEnemiesSpawned 0)
      (for _array_element (Utilities|Struct|BreakWaveInfo _returnvalue)
        (Variables|Default|SetEnemiesSpawned (+ (Variables|Default|GetEnemiesSpawned) (.EnemyNumber (Utilities|Struct|BreakEnemyInfo _array_element)))))
      (Variables|Default|SetWaveInfoMax (Utilities|Array|Length (Utilities|Struct|BreakWaveInfo _returnvalue)))
      (Variables|Default|SetWaveInfoIndex 0)
      (Variables|Default|SetKilledEnemyAmount 0)
      (bind _returnvalue_2 (Utilities|Time|SetTimerbyFunctionName 0 "Spawn Enemies" (Variables|Default|GetTimeBetweenSpawn) true 0.1))
      (Variables|Default|SetSpawnEnemyTimerHandle _returnvalue_2))
    (:RowNotFound
      (Development|PrintString "Couldn't find row for wave data"))))

(event Custom|Start%20Checking%20If%20Enemies%20Are%20Dead
  ;[1 1 1] Check if enemies are dead, and start new wave
)

(event EventBeginPlay
  ;[1 1 1] Sort enemy spawner references
  (bind _outactors (Actor|GetAllActorsOfClass "/Game/Blueprints/WaveSystem/BP_WaveSpawnPoint.BP_WaveSpawnPoint_C"))
  (bind _output_get (Variables|Default|SetEnemySpawnPoints _outactors))
  (for _array_element _output_get
    (switch Utilities|FlowControl|Switch|SwitchonE_EnemyType (Variables|/Game/Blueprints/WaveSystem/BP_WaveSpawnPoint.BP_WaveSpawnPoint_C|GetSpawnerType _array_element)
      (:NewEnumerator0
        (Utilities|Array|Add (Variables|Default|GetE_Ground) _array_element))))
  (CallFunction|StartCountdown))

(fn ConstructionScript)

(fn SpawnEnemies
  (bind _waveinfoindex (Variables|Default|GetWaveInfoIndex))
  (bind _currentwaveinfo (Variables|Default|GetCurrentWaveInfo))
  (bind _output (Utilities|Array|Get(acopy) _currentwaveinfo _waveinfoindex))
  (bind (_enemyclass _enemynumber _enemytype) (Utilities|Struct|BreakEnemyInfo _output))
  (if (< (Variables|Default|GetWaveInfoIndex) (Variables|Default|GetWaveInfoMax)) :!label _label
    (if (< (Variables|Default|GetamountOfEnemyOfTypedSpawned) _enemynumber)
      (bind _output_get (LocalVariables|SetCurrent%20Spawn%20Points (Utilities|Select :Index _enemytype :NewEnumerator0 (Variables|Default|GetE_Ground))))
      (bind _asbp_throwing_enemy (Utilities|Casting|CastToBP_ThrowingEnemyClass _enemyclass))
      (bind _returnvalue (CallFunction|GetSpawnPoints _output_get))
      (Game|SpawnActorfromClass _asbp_throwing_enemy _returnvalue "Undefined" 0 self 0)
      (Math|Integer|IncrementInt (Variables|Default|GetamountOfEnemyOfTypedSpawned))
      (else
        (Math|Integer|IncrementInt (Variables|Default|GetWaveInfoIndex)
          (:%20%20
            (Variables|Default|SetamountOfEnemyOfTypedSpawned 0)
            (goto _label)))))
    (else
      (Utilities|Time|ClearandInvalidateTimerbyHandle (Variables|Default|GetSpawnEnemyTimerHandle))
      (Math|Integer|IncrementInt (Variables|Default|GetWaveCounter)))))

(fn EnemyDead
  (Math|Integer|IncrementInt (Variables|Default|GetKilledEnemyAmount)
    (:%20%20
      (CallFunction|CheckWaveEnd))))

(fn GetSpawnPoints
  (params (CurrentSpawnPoints :type Array%20of%20BP%20Wave%20Spawn%20Point%20Object%20References))
  (return (Transformation|GetWorldTransform (Variables|/Game/Blueprints/WaveSystem/BP_WaveSpawnPoint.BP_WaveSpawnPoint_C|GetBillboard (Utilities|Array|Get(acopy) CurrentSpawnPoints (Math|Random|RandomIntegerinRange 0 (Utilities|Array|LastIndex CurrentSpawnPoints)))))))

(fn CheckWaveEnd
  (if (>= (Variables|Default|GetKilledEnemyAmount) (Variables|Default|GetEnemiesSpawned))
    (CallFunction|StartCountdown)))

(fn GameComplete
  (bind _returnvalue (Utilities|GetDataTableRow (Variables|Default|GetEnemyDataTable) (Utilities|String|StringToName (Utilities|String|ToString(Integer) (Variables|Default|GetWaveCounter))))
    (:then
      (return false))
    (:RowNotFound
      (return true))))