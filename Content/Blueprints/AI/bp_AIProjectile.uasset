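; AI projectile actor that deals damage on hit to actors with a HealthComponent.
; On spawn it ignores its owner while moving, clears HasHitObject and destroys itself after a fixed lifetime.
; Mesh hits act only when HasHitObject is true, yet the flag starts false and is set only inside that branch.
; Damage credits the owner's AI controller and destroys the projectile.
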(event OnComponentHit(ProjectileMesh)
  (params (HitComponent :type Primitive%20Component%20Object%20Reference) (OtherActor :type Actor%20Object%20Reference) (OtherComp :type Primitive%20Component%20Object%20Reference) (NormalImpulse :type Vector :default "0, 0, 0") (Hit :type Hit%20Result%20Structure%20%28by%20ref%29))
  (bind _returnvalue (Actor|GetComponentbyClass OtherActor "/Script/BrackeysGameJam2020.HealthComponent"))
  (if (Variables|Default|GetbHasHitObject)
    (Utilities|IsValid _returnvalue
      (:Is%20Valid
        (Class|HealthComponent|DealDamage _returnvalue OtherActor (Variables|Default|GetProjectileDamage) (AI|GetAIController (Components|GetOwner)) "0, 0, 0" self)
        (Actor|DestroyActor))
      (:Is%20Not%20Valid
        (Variables|Default|SetbHasHitObject true)))))

(event EventBeginPlay
  (Collision|IgnoreActorwhenMoving (Variables|Default|GetProjectileMesh) (Components|GetOwner) true)
  (Variables|Default|SetbHasHitObject false)
  (Utilities|FlowControl|Delay 1e+01)
  (Actor|DestroyActor))

(fn ConstructionScript)