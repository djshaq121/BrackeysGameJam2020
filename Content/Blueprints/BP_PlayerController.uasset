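; Player controller that handles the player's death and switches to the quit screen.
; On begin play it sets game-only input and binds to the BP_Player health component's change event.
; The first death clears widgets, shows BP_QuitScreenWidget with the mouse cursor, disables pawn input and hides the dodgeball.
; It also spawns BP_DeathCamera at the player camera's transform and makes it the view target, dropping the view to the ground.
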(event Custom|HealthChange
  (params (HealthComp :type Health%20Component%20Object%20Reference) (Health :type Float%20%28single-precision%29) (HitImpactPoint :type Vector) (InstigatedBy :type Controller%20Object%20Reference) (DamageCauser :type Actor%20Object%20Reference))
  (bind _self self)
  (if (and (Class|HealthComponent|GetIsDead HealthComp) (not (Variables|Default|GetbPlayerHasDied)))
    (Variables|Default|SetbPlayerHasDied true)
    (Viewport|RemoveAllWidgets)
    (bind _returnvalue (UserInterface|CreateWidget "/Game/MainMenu/BP_QuitScreenWidget.BP_QuitScreenWidget_C" self))
    (UserInterface|Viewport|AddtoViewport _returnvalue 0)
    (Input|DisableInput (Variables|Default|GetControlledPlayer) _self)
    (Variables|Default|SetbShowMouseCursor true)
    (Input|SetInputModeGameandUI _self _returnvalue "DoNotLock" true)
    ;[1 1 1] Drop camera to the ground
    (CallFunction|SpawnDeathCamera)
    (Development|SetHiddeninGame (Variables|/Game/Blueprints/BP_Player.BP_Player_C|GetDodgeBall (Variables|Default|GetControlledPlayer)) true false)))

(event EventBeginPlay
  (bind _asbp_player (Utilities|Casting|CastToBP_Player (Game|Player|GetPlayerPawn 0)))
  (bind _output_get (Variables|Default|SetControlledPlayer _asbp_player))
  (EventDispatchers|BindEventtoOnHealthChange (Variables|/Game/Blueprints/BP_Player.BP_Player_C|GetHealth _output_get) (delegate Custom|HealthChange))
  (Variables|Default|SetbPlayerHasDied false)
  (Variables|Default|SetbShowMouseCursor false)
  (Input|SetInputModeGameOnly self))

(event EventTick
  (params (DeltaSeconds :type Float%20%28single-precision%29)))

(fn ConstructionScript)

(fn SpawnDeathCamera
  (bind _controlledplayer (Variables|Default|GetControlledPlayer))
  (bind _returnvalue (Actor|GetComponentbyClass _controlledplayer "/Script/Engine.CameraComponent"))
  (Utilities|IsValid _returnvalue
    (:Is%20Valid
      (bind _returnvalue_2 (Game|SpawnActorfromClass "/Game/Blueprints/BP_DeathCamera.BP_DeathCamera_C" (Math|Transform|MakeTransform (Transformation|GetWorldLocation _returnvalue) (Transformation|GetWorldRotation _returnvalue) "1,1,1") "Undefined" 0 0))
      (Game|Player|SetViewTargetwithBlend _returnvalue_2 0.0 "VTBlend_Linear" 0.0 true))))