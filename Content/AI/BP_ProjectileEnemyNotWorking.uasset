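; Projectile-throwing enemy that plays a throw montage at a given target when Attack is called.
; SpawnProjectile attaches a scaled-down BP_AIProjectile to a mesh socket with collision and movement stopped.
; ThrowProjectile detaches it, restores collision and sets velocity from the unnormalized target offset plus vertical aim offset, times ProjectileSpeed, so speed scales with distance.
; Nothing in this graph calls the spawn or throw events.
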(event EventThrowProjectile
  (Utilities|IsValid (Variables|Default|GetProjectileSpawned)
    (:Is%20Valid
      (Physics|SetSimulatePhysics (Variables|/Game/AI/BP_AIProjectile.BP_AIProjectile_C|GetProjectileMesh (Variables|Default|GetProjectileSpawned)) false)
      (Transformation|DetachFromComponent (Variables|/Script/Engine.Actor|GetRootComponent (Variables|Default|GetProjectileSpawned)) "KeepWorld" "KeepWorld" "KeepWorld" true)
      (Collision|SetCollisionEnabled (Variables|/Game/AI/BP_AIProjectile.BP_AIProjectile_C|GetProjectileMesh (Variables|Default|GetProjectileSpawned)) "QueryAndPhysics")
      (Variables|/Script/Engine.MovementComponent|SetVelocity (Variables|/Game/AI/BP_AIProjectile.BP_AIProjectile_C|GetProjectileMovement (Variables|Default|GetProjectileSpawned)) (* (+ (- (Transformation|GetActorLocation (Variables|Default|GetTargetToAttack)) (Transformation|GetActorLocation (Variables|Default|GetProjectileSpawned))) (* (Math|Vector|VectorUp) (Variables|Default|GetzAimOffset))) (Variables|Default|GetProjectileSpeed))))))

(event EventSpawnProjectile
  (bind _self self)
  (bind _returnvalue (Game|SpawnActorfromClass "/Game/AI/BP_AIProjectile.BP_AIProjectile_C" (Math|Transform|MakeTransform (Transformation|GetSocketLocation (Variables|Character|GetMesh) (Variables|Default|GetSpawnProjectileSocketName)) "0, 0, 0" "0.300000,0.300000,0.300000") "Undefined" _self _self))
  (bind _output_get (Variables|Default|SetProjectileSpawned _returnvalue))
  (Collision|SetCollisionEnabled (Variables|/Game/AI/BP_AIProjectile.BP_AIProjectile_C|GetProjectileMesh _output_get) "NoCollision")
  (Components|Movement|StopMovementImmediately (Variables|/Game/AI/BP_AIProjectile.BP_AIProjectile_C|GetProjectileMovement (Variables|Default|GetProjectileSpawned)))
  (Transformation|AttachComponentToComponent (Variables|Default|GetProjectileSpawned) (Variables|Character|GetMesh) (Variables|Default|GetSpawnProjectileSocketName) "SnapToTarget" "SnapToTarget" "KeepRelative" true))

(event EventAttack
  (params (TargetToAttack :type Actor%20Object%20Reference))
  (Variables|Default|SetTargetToAttack TargetToAttack)
  (Animation|Montage|PlayMontage (Variables|Character|GetMesh) "/Game/AI/Animations/Throw_Montage.Throw_Montage"))

(fn ConstructionScript)