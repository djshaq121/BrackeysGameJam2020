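; BP_ThrowingEnemy is an AI enemy that plays a throw montage when told to attack a target.
; Separate events spawn a projectile attached to a hand-style mesh socket with collision off, then detach it, restore collision and activate its movement if the target is valid.
; The target-aimed velocity calculation is unconnected.
; Zero health triggers ragdoll, and destruction notifies the wave manager of the death.
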(event OnHealthChange(HealthComponent)
  (params (HealthComp :type Health%20Component%20Object%20Reference) (Health :type Float%20%28single-precision%29) (HitDirection :type Vector :default "0, 0, 0") (InstigatedBy :type Controller%20Object%20Reference) (DamageCauser :type Actor%20Object%20Reference))
  (if (<= Health 0.0)
    (Class|RagdollComponent|Ragdoll (Variables|Default|GetRagdoll))))

(event EventThrowProjectile
  (bind _projectilespawned (Variables|Default|GetProjectileSpawned))
  (bind _projectilespawned_2 (Variables|Default|GetProjectileSpawned))
  (Utilities|IsValid _projectilespawned_2
    (:Is%20Valid
      (Physics|SetSimulatePhysics (Variables|/Script/BrackeysGameJam2020.ProjectileBase|GetStaticMesh _projectilespawned_2) false)
      (Transformation|DetachFromComponent (Variables|/Script/Engine.Actor|GetRootComponent (Variables|Default|GetProjectileSpawned)) "KeepWorld" "KeepWorld" "KeepWorld" true)
      (Utilities|IsValid _projectilespawned
        (:Is%20Valid
          (Collision|SetCollisionEnabled (Variables|/Script/BrackeysGameJam2020.ProjectileBase|GetStaticMesh _projectilespawned) "QueryAndPhysics")
          (Utilities|IsValid (Variables|Default|GetTargetToAttack)
            (:Is%20Valid
              (Components|Activation|Activate (Variables|/Game/AI/BP_AIProjectile.BP_AIProjectile_C|GetProjectileMovement (Variables|Default|GetProjectileSpawned)) false))))))))

(event EventDestroyed
  (bind _wavemangerref (Variables|Default|GetWaveMangerRef))
  (Utilities|IsValid _wavemangerref
    (:Is%20Valid
      (Default|EnemyDead _wavemangerref))))

(event EventAttack
  (params (TargetToAttack :type Actor%20Object%20Reference))
  (Variables|Default|SetTargetToAttack TargetToAttack)
  (Animation|Montage|PlayMontage (Variables|Character|GetMesh) "/Game/AI/Animations/Throw_Montage.Throw_Montage"))

(event EventSpawnProjectile
  (bind _self self)
  (bind _returnvalue (Game|SpawnActorfromClass "/Game/AI/BP_AIProjectile.BP_AIProjectile_C" (Math|Transform|MakeTransform (Transformation|GetSocketLocation (Variables|Character|GetMesh) (Variables|Default|GetSpawnProjectileSocketName)) (Transformation|GetActorRotation) "0.300000,0.300000,0.300000") "Undefined" _self _self))
  (bind _output_get (Variables|Default|SetProjectileSpawned _returnvalue))
  (Collision|SetCollisionEnabled (Variables|/Script/BrackeysGameJam2020.ProjectileBase|GetStaticMesh _output_get) "NoCollision")
  (Utilities|IsValid (Variables|Default|GetProjectileSpawned)
    (:Is%20Valid
      (Transformation|AttachComponentToComponent (Variables|Default|GetProjectileSpawned) (Variables|Character|GetMesh) (Variables|Default|GetSpawnProjectileSocketName) "SnapToTarget" "SnapToTarget" "KeepRelative" true))))

(fn ConstructionScript)